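; BP_FlameThrower is a short-lived flamethrower effect Blueprint in the rocket-back folder, built from a static mesh and two Niagara components.
; On BeginPlay it activates both Niagara systems without a reset, waits a fixed three-second delay, then destroys the mesh and both effects.
; Only the components are destroyed, with no explicit destroy of the actor itself, and the graph contains no overlap, damage or tick logic.
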(event `self.ReceiveBeginPlay`
  (`ActorComponent.Activate` (`self.Niagara`) false)
  (`ActorComponent.Activate` (`self.Niagara1`) false)
  (`KismetSystemLibrary.Delay` 3.0)
  (`ActorComponent.K2_DestroyComponent` (`self.StaticMesh`))
  (`ActorComponent.K2_DestroyComponent` (`self.Niagara`))
  (`ActorComponent.K2_DestroyComponent` (`self.Niagara1`)))

(fn `UserConstructionScript`)