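; BP_Player is the player Blueprint handling backpack input and gunpowder-limited flight.
; BeginPlay creates the backpack and "cannot fly" widgets, and a FlipFlop-driven event shows or hides the backpack along with the mouse cursor.
; The flight input spends one gunpowder to call UpFly, or shows the warning widget for a few seconds when none remains.
; A debug F key calls ShowMouse.
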(event Custom|backpack_operation
  (bind _returnvalue (Game|GetPlayerController 0))
  ;[0.15 0.15 0.15 0.5] 背包打开或关闭
  (Utilities|FlowControl|FlipFlop
    (:A
      (UserInterface|Viewport|AddtoViewport (Variables|Default|Getbackpack) 0)
      (Variables|Default|Setback_pack_opean? true)
      (Variables|/Script/Engine.PlayerController|SetbShowMouseCursor _returnvalue true))
    (:B
      (Widget|RemovefromParent (Variables|Default|Getbackpack))
      (Variables|Default|Setback_pack_opean? false)
      (Variables|/Script/Engine.PlayerController|SetbShowMouseCursor _returnvalue false))))

(event Input|EnhancedActionEvents|EnhancedInputActionPlayer_backpack
  (params (ActionValue :type Boolean) (ElapsedSeconds :type Float%20%28double-precision%29) (TriggeredSeconds :type Float%20%28double-precision%29) (InputAction :type Input%20Action%20Object%20Reference :default "/Game/BluePrint/Input/Player_backpack.Player_backpack"))
  ;[0.15 0.15 0.15 0.5] 背包打开或关闭
  (CallFunction|BackpackOperation))

(event Input|EnhancedActionEvents|EnhancedInputActionPlayer_Flying
  (params (ActionValue :type Boolean) (ElapsedSeconds :type Float%20%28double-precision%29) (TriggeredSeconds :type Float%20%28double-precision%29) (InputAction :type Input%20Action%20Object%20Reference :default "/Game/BluePrint/Input/Player_Flying.Player_Flying"))
  (bind _cannot_fly (Variables|Default|Getcannot_fly))
  ;[0.15 0.15 0.15 0.5] 能否飞行
  (if (> (Variables|Default|Getgunpower_cont) 0)
    (Variables|Default|Setgunpower_cont (- (Variables|Default|Getgunpower_cont) 1))
    (Class|MainPlayer|UpFly)
    (else
      (UserInterface|Viewport|AddtoViewport _cannot_fly 0)
      (Utilities|FlowControl|Delay 4.0)
      (Widget|RemovefromParent _cannot_fly))))

(event EventBeginPlay
  ;[0.15 0.15 0.15 0.5] 初始化
  (bind _returnvalue (UserInterface|CreateWidget "/Game/BluePrint/UI/backpack/backpack_bg.backpack_bg_C"))
  (Variables|Default|Setbackpack _returnvalue)
  (bind _returnvalue_2 (UserInterface|CreateWidget "/Game/BluePrint/UI/backpack/cannot_fly.cannot_fly_C"))
  (Variables|Default|Setcannot_fly _returnvalue_2))

(event Input|KeyboardEvents|DebugKeyF
  (params (Key :type Key%20Structure :default "None") (ActionValue :type Input%20Action%20Value%20Structure))
  (:Pressed
    (Class|MainPlayer|ShowMouse)))

(fn ConstructionScript)