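; LuBanLockTest is a keyboard test Blueprint for triggering the pieces of a Luban lock puzzle.
; Keys 1 to 5 each find the matching Lock1 to Lock5 actor by class, cast it and call MoveTheLock.
; Unconnected leftover nodes would set CanMove on Lock2 through Lock5, most behind a CanMove check, but they never run.
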(event `self.ReceiveBeginPlay`)

(event `self.ReceiveTick`
  (params (DeltaSeconds :type "Float (single-precision)")))

(event `Key|One`
  (params (Key :type "Key Structure"))
  (:`Pressed`
    (bind _returnvalue (`GameplayStatics.GetActorOfClass` "/Game/BluePrint/LuBanLock/Lock1.Lock1_C"))
    (bind _aslock_1 (cast `/Game/BluePrint/LuBanLock/Lock1` _returnvalue))
    (`LuBanLock.MoveTheLock` _aslock_1)))

(event `Key|Two`
  (params (Key :type "Key Structure"))
  (:`Pressed`
    (bind _returnvalue (`GameplayStatics.GetActorOfClass` "/Game/BluePrint/LuBanLock/Lock2.Lock2_C"))
    (bind _aslock_2 (cast `/Game/BluePrint/LuBanLock/Lock2` _returnvalue))
    (`LuBanLock.MoveTheLock` _aslock_2)))

(event `Key|Three`
  (params (Key :type "Key Structure"))
  (:`Pressed`
    (bind _returnvalue (`GameplayStatics.GetActorOfClass` "/Game/BluePrint/LuBanLock/Lock3.Lock3_C"))
    (bind _aslock_3 (cast `/Game/BluePrint/LuBanLock/Lock3` _returnvalue))
    (`LuBanLock.MoveTheLock` _aslock_3)))

(event `Key|Four`
  (params (Key :type "Key Structure"))
  (:`Pressed`
    (bind _returnvalue (`GameplayStatics.GetActorOfClass` "/Game/BluePrint/LuBanLock/Lock4.Lock4_C"))
    (bind _aslock_4 (cast `/Game/BluePrint/LuBanLock/Lock4` _returnvalue))
    (`LuBanLock.MoveTheLock` _aslock_4)))

(event `Key|Five`
  (params (Key :type "Key Structure"))
  (:`Pressed`
    (bind _returnvalue (`GameplayStatics.GetActorOfClass` "/Game/BluePrint/LuBanLock/Lock5.Lock5_C"))
    (bind _aslock_5 (cast `/Game/BluePrint/LuBanLock/Lock5` _returnvalue))
    (`LuBanLock.MoveTheLock` _aslock_5)))

(fn `UserConstructionScript`)