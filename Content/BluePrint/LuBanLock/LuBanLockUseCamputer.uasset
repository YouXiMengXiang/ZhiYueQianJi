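; Interactable computer actor that lets the player switch control to the LuBan lock puzzle pawn.
; Overlap by BP_Player shows a prompt widget and enables the C key; ending overlap on the Re component hides and disables it.
; C flip-flops possession between BP_LuBanLockPlayer and BP_Player, both found by class, showing or closing the mouse cursor accordingly.
; The control UI creation is unconnected and never runs.
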(event `self.ReceiveBeginPlay`
  (`SceneComponent.SetVisibility` (`self.Widget`) false false))

(event `self.ReceiveActorBeginOverlap`
  (params (OtherActor :type "Actor Object Reference"))
  (cast `/Game/BluePrint/Player/BP_Player` OtherActor)
  (`SceneComponent.SetVisibility` (`self.Widget`) true false)
  (set `self.PlayerIsControl` true))

(event `self.re.OnComponentEndOverlap`
  (params (OverlappedComponent :type "PrimitiveComponent Object Reference") (OtherActor :type "Actor Object Reference") (OtherComp :type "PrimitiveComponent Object Reference") (OtherBodyIndex :type Integer))
  (cast `/Game/BluePrint/Player/BP_Player` OtherActor)
  (`SceneComponent.SetVisibility` (`self.Widget`) false false)
  (set `self.PlayerIsControl` false))

(event `Key|C`
  (params (Key :type "Key Structure"))
  (:`Pressed`
    (if (`self.PlayerIsControl`)
      (`/Engine/EditorBlueprintResources/StandardMacros.FlipFlop`
        (:`A`
          (bind _returnvalue (`GameplayStatics.GetActorOfClass` "/Game/BluePrint/Player/BP_LuBanLockPlayer.BP_LuBanLockPlayer_C"))
          (bind _asbp_lu_ban_lock_player (cast `/Game/BluePrint/Player/BP_LuBanLockPlayer` _returnvalue))
          (`Controller.Possess` (`GameplayStatics.GetPlayerController` 0) _asbp_lu_ban_lock_player)
          (`LuBanLockPlayer.ShowMouse` _asbp_lu_ban_lock_player))
        (:`B`
          (bind _returnvalue_2 (`GameplayStatics.GetActorOfClass` "/Game/BluePrint/Player/BP_Player.BP_Player_C"))
          (bind _asbp_player (cast `/Game/BluePrint/Player/BP_Player` _returnvalue_2))
          (`Controller.Possess` (`GameplayStatics.GetPlayerController` 0) _asbp_player)
          (`MainPlayer.CloseMouse` _asbp_player))))))

(fn `UserConstructionScript`)