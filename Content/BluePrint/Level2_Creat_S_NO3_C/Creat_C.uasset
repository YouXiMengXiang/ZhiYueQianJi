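; Level 2 spawner actor that produces C_tan_actor instances at its own location while the spot is clear.
; It spawns one at BeginPlay, then a looping timer retries Create every few seconds.
; A CanCreate flag gates spawning, cleared when a C_tan_actor overlaps the actor and set again when one leaves the Box component.
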(event `self.ReceiveBeginPlay`
  (set `self.CanCreate` true)
  (`self.Create`)
  (`KismetSystemLibrary.K2_SetTimer` null "Create" 5.0 true))

(event `self.ReceiveActorBeginOverlap`
  (params (OtherActor :type "Actor Object Reference"))
  (cast `/Game/BluePrint/UI/backpack/C_tan_actor` OtherActor)
  (set `self.CanCreate` false))

(event `self.Box.OnComponentEndOverlap`
  (params (OverlappedComponent :type "PrimitiveComponent Object Reference") (OtherActor :type "Actor Object Reference") (OtherComp :type "PrimitiveComponent Object Reference") (OtherBodyIndex :type Integer))
  (cast `/Game/BluePrint/UI/backpack/C_tan_actor` OtherActor)
  (set `self.CanCreate` true))

(fn `Create`
  (if (`self.CanCreate`)
    (`|SpawnActorFromClass` "/Game/BluePrint/UI/backpack/C_tan_actor.C_tan_actor_C" (`KismetMathLibrary.Conv_VectorToTransform` (`self.K2_GetActorLocation` self)) "Undefined" "MultiplyWithRoot" null null)))

(fn `UserConstructionScript`)