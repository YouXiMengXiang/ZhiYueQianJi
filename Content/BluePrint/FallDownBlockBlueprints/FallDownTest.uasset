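; FallDownTest is a Blueprint that arms a delayed fall flag once a linked FallDownBoll ball has fallen.
; BeginPlay casts the FallDownBall reference, caches it and enables the check only if the cast succeeds.
; Tick polls the ball's BollFallDown flag and, after a short Delay, sets CanFallDown, which nothing in this graph reads or resets.
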(event `self.ReceiveBeginPlay`
  (bind _asfall_down_boll (cast `FallDownBoll` (`self.FallDownBall`)))
  (set `self.IsOk` true)
  (set `self.As Fall Down Boll` _asfall_down_boll))

(event `self.ReceiveTick`
  (params (DeltaSeconds :type "Float (single-precision)"))
  (if (`self.IsOk`)
    (if (`FallDownBoll.BollFallDown` (`self.As Fall Down Boll`))
      (`KismetSystemLibrary.Delay` 2.0)
      (set `self.CanFallDown` true))))

(fn `UserConstructionScript`)